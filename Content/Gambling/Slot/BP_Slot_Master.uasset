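; BP_Slot_Master is a slot machine that shows three random values and can award chips to the player.
; Interact sets three text displays from random Values entries, then HandleWin adds 1000 to BP_GamblingAddict's PlayerChips if the displays compare equal.
; That check compares the Value1–3 references themselves, not their text, and no stake is deducted.
; Prompt events toggle a widget's visibility, while Interactable always returns false.
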(event Custom|Handle%20Win
  (bind _value_2 (Variables|Default|GetValue%202))
  (if (and (== (Variables|Default|GetValue%201) _value_2) (== _value_2 (Variables|Default|GetValue%203)))
    (bind _asbp_gambling_addict (Utilities|Casting|CastToBP_GamblingAddict (Game|GetPlayerCharacter 0)))
    (Variables|/Game/Character/Blueprints/BP_GamblingAddict.BP_GamblingAddict_C|SetPlayerChips _asbp_gambling_addict (+ (Variables|/Game/Character/Blueprints/BP_GamblingAddict.BP_GamblingAddict_C|GetPlayerChips _asbp_gambling_addict) 1000))))

(event EventInteractPrompt
  (Rendering|SetVisibility (Variables|Default|GetWidget) true false))

(event EventRemoveInteractPrompt
  (Rendering|SetVisibility (Variables|Default|GetWidget) false false))

(event EventInteract
  (bind _values (Variables|Default|GetValues))
  (bind _outitem (Utilities|Array|Random _values))
  (Rendering|Components|TextRender|SetText (Variables|Default|GetValue%201) _outitem)
  (Rendering|Components|TextRender|SetText (Variables|Default|GetValue%202) _outitem)
  (Rendering|Components|TextRender|SetText (Variables|Default|GetValue%203) _outitem)
  (CallFunction|HandleWin))

(fn ConstructionScript)

(fn Interactable
  (params (Interactable :type Boolean))
  (return false))