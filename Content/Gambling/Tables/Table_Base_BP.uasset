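; Base Blueprint for gambling tables, where interacting seats the player's GamblingAddict character at the minimum bet and records starting bet and chips.
; Start, Split, Stand, Hit, Double and End form the game-action events, all empty except Double, which subtracts the starting bet from game chips.
; A helper function line-traces from the table camera, with persistent debug drawing, to add or remove the interact-dot widget.
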(event EventDouble
  (Variables|Default|SetPlayer%20Game%20Chips (- (Variables|Default|GetPlayer%20Game%20Chips) (Variables|Default|GetPlayer%20Starting%20Bet))))

(event EventEnd)

(event EventInteract
  ;[0.15 0.15 0.15 0.5] Sit At Table
  (bind _asbp_gambling_addict (Utilities|Casting|CastToBP_GamblingAddict (Game|GetPlayerCharacter 0)))
  (Variables|/Game/Character/Blueprints/BP_GamblingAddict.BP_GamblingAddict_C|SetisSat _asbp_gambling_addict true)
  (Variables|/Game/Character/Blueprints/BP_GamblingAddict.BP_GamblingAddict_C|SetPlayerBet _asbp_gambling_addict (Variables|Default|GetTable%20Minimum%20Bet))
  (Variables|Default|SetPlayer%20Starting%20Bet (Variables|/Game/Character/Blueprints/BP_GamblingAddict.BP_GamblingAddict_C|GetPlayerBet _asbp_gambling_addict))
  (Variables|Default|SetPlayer%20Starting%20Chips (Variables|/Game/Character/Blueprints/BP_GamblingAddict.BP_GamblingAddict_C|GetPlayerChips _asbp_gambling_addict)))

(event EventStart)

(event EventHit)

(event EventStand)

(event EventSplit)

(fn ConstructionScript)

(fn HidetheSillyDot,andSometimesBringItBack
  (bind _interact_dot (Variables|Default|GetInteract%20Dot))
  (bind _returnvalue (UserInterface|Viewport|IsinViewport _interact_dot))
  (Variables|Default|GetInteract%20Dot
    (:then
      (Variables|Default|SetTable-Cam (Variables|Default|GetTable-Cam))
      (bind (_outhit _returnvalue_2) (Collision|LineTraceByChannel (Transformation|GetWorldLocation (Variables|Default|GetTable-Cam)) (+ (Transformation|GetWorldLocation (Variables|Default|GetTable-Cam)) (* (Math|Vector|GetForwardVector (Variables|Default|GetTable-Cam)) 3e+02)) "TraceTypeQuery1" false 0 "Persistent"))
      (if _returnvalue_2
        (bind _astable_base_bp (Utilities|Casting|CastToTable_Base_BP (.HitActor (Collision|BreakHitResult _outhit)))
          (:then
            (if (and (Utilities|DoesObjectImplementInterface (.HitActor (Collision|BreakHitResult _outhit)) "/Game/Character/InteractInterface.InteractInterface_C") (Variables|Table_Base_BP_C|GetInteractable_0 _astable_base_bp))
              (if (not _returnvalue) :!label _label
                (UserInterface|Viewport|AddtoViewport _interact_dot 0))
              (else
                (if _returnvalue :!label _label_2
                  (Default|Remove _interact_dot)))))
          (:CastFailed
            (goto _label)))
        (else
          (goto _label_2))))
    (:else)))

(fn Interactable
  (params (Interactable :type Boolean))
  (return false))